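; BP_PlayerSpacecraft is the player spacecraft Blueprint, adding debug and temporary test key bindings on top of its parent class.
; T toggles fast global time dilation through a FlipFlop.
; C and X each toggle a video or audio settings widget, switching input to Game and UI on open.
; Closing either removes all widgets without restoring the input mode, and the variable names mark the widgets for later deletion.
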(event `self.ReceiveBeginPlay`
  (`parent.ReceiveBeginPlay`))

(event `Key|T`
  (params (Key :type "Key Structure"))
  ;[1 1 1] For debug
  (:`Pressed`
    (`/Engine/EditorBlueprintResources/StandardMacros.FlipFlop`
      (:`A`
        (`GameplayStatics.SetGlobalTimeDilation` 4.0))
      (:`B`
        (`GameplayStatics.SetGlobalTimeDilation` 1.0)))))

(event `Key|C`
  (params (Key :type "Key Structure"))
  (bind _returnvalue (`GameplayStatics.GetPlayerController` 0))
  ;[1 1 1] For debug
  (:`Pressed`
    (`/Engine/EditorBlueprintResources/StandardMacros.FlipFlop`
      (:`A`
        (bind _returnvalue_2 (`|CreateWidget` "/Game/UI/Settings/HeaderMenuTabs/VideoSettings/WBP_VideoSettings.WBP_VideoSettings_C" _returnvalue))
        (bind _output_get (set `self.VideoSetting_THEN_DELETE` _returnvalue_2))
        (`UserWidget.AddToViewport` _output_get 0)
        (`WidgetBlueprintLibrary.SetInputMode_GameAndUIEx` _returnvalue _output_get "DoNotLock" false))
      (:`B`
        (`WidgetLayoutLibrary.RemoveAllWidgets`)))))

(event `Key|X`
  (params (Key :type "Key Structure"))
  (bind _returnvalue (`GameplayStatics.GetPlayerController` 0))
  ;[1 1 1] For debug
  (:`Pressed`
    (`/Engine/EditorBlueprintResources/StandardMacros.FlipFlop`
      (:`A`
        (bind _returnvalue_2 (`|CreateWidget` "/Game/UI/Settings/HeaderMenuTabs/AudioSettings/WBP_AudioSettingsWidget.WBP_AudioSettingsWidget_C" _returnvalue))
        (bind _output_get (set `self.AudioSetting_THEN_DELETE` _returnvalue_2))
        (`UserWidget.AddToViewport` _output_get 0)
        (`WidgetBlueprintLibrary.SetInputMode_GameAndUIEx` _returnvalue _output_get "DoNotLock" false))
      (:`B`
        (`WidgetLayoutLibrary.RemoveAllWidgets`)))))

(fn `UserConstructionScript`)