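; Base asteroid Blueprint that adds visual and audio feedback to the death and hit events of its parent class.
; On death it calls the parent handler, hides the actor rather than destroying it here, and spawns the DeathEffect Niagara system at its location and rotation.
; On a visual hit event it calls the parent handler, then plays the hit sound at the asteroid's location.
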(event `self.OnDeath`
  ;[0 0 0] OnDeath_Visual
  (`parent.OnDeath`)
  (`self.SetActorHiddenInGame` true)
  (`NiagaraFunctionLibrary.SpawnSystemAtLocation` (`self.DeathEffect`) (`self.K2_GetActorLocation`) (`self.K2_GetActorRotation`)))

(event `self.OnAsteroidHit_Visual`
  ;[0 0 0] OnAsteroidHit_Visual
  (`parent.OnAsteroidHit_Visual`)
  (`GameplayStatics.PlaySoundAtLocation` (`self.SoundHit`) (`self.K2_GetActorLocation`) (`self.K2_GetActorRotation`) 1.0 1.0 0.0 null null null null))

(fn `UserConstructionScript`)