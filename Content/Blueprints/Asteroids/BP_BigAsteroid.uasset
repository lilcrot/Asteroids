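; Big asteroid that breaks into two small asteroids when it dies, after running the parent death logic.
; SplitUpToSmallAsteroids spawns each BP_SmallAsteroid at a random distance and angle within a cone around the forward vector, with Z zeroed to keep the offset horizontal.
; Spawn rotation comes from the same random vector expression, and collision handling nudges a blocked spawn or skips it.
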(event `self.OnDeath`
  (`parent.OnDeath`)
  (`self.SplitUpToSmallAsteroids` 2))

(fn `SplitUpToSmallAsteroids`
  (params (SmallAsteroidsNumber :type Integer :default 1))
  (locals (MinConeHalfAngle :type "Float (double-precision)" :default 30.0) (MaxConeHalfAngle :type "Float (double-precision)" :default 150.0) (MinDistance :type "Float (double-precision)" :default 150.0) (MaxDistance :type "Float (double-precision)" :default 300.0))
  (bind (_returnvalue_x _returnvalue_y _returnvalue_z) (`KismetMathLibrary.BreakVector` (`KismetMathLibrary.RandomUnitVectorInConeInDegrees` (`self.GetActorForwardVector`) (`KismetMathLibrary.RandomFloatInRange` (`local.MinConeHalfAngle`) (`local.MaxConeHalfAngle`)))))
  (bind _returnvalue (* (`KismetMathLibrary.MakeVector` _returnvalue_x _returnvalue_y (* _returnvalue_z 0.0)) (`KismetMathLibrary.RandomFloatInRange` (`local.MinDistance`) (`local.MaxDistance`))))
  (for _ (range 1 (+ SmallAsteroidsNumber 1))
    (`|SpawnActorFromClass` "/Game/Blueprints/Asteroids/BP_SmallAsteroid.BP_SmallAsteroid_C" (`KismetMathLibrary.MakeTransform` (+ (`self.K2_GetActorLocation`) _returnvalue) (`KismetMathLibrary.Conv_VectorToRotator` _returnvalue)) "AdjustIfPossibleButDontSpawnIfColliding" "MultiplyWithRoot" null self)))

(fn `UserConstructionScript`)